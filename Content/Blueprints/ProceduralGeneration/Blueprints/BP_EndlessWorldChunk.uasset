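; BP_EndlessWorldChunk extends an endless world around the player by placing instanced static mesh tiles on a flat chunk grid.
; Tick compares the player's chunk coordinates with the last known ones.
; On entering an unvisited chunk, it adds instances across the square render range and records that coordinate in Grid.
; Grid tracks only visited centres, so overlapping ranges add duplicate instances, and none are removed.
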(event EventBeginPlay)

(event Collision|EventActorBeginOverlap
  (params (OtherActor :type Actor%20Object%20Reference)))

(event EventTick
  (params (DeltaSeconds :type Float%20%28single-precision%29))
  (bind _coordinates (Utilities|GetChunkCoordinates))
  (if (not (and (== (.x _coordinates) (.x (Variables|Default|GetLastKnownPlayerCoor))) (== (.y _coordinates) (.y (Variables|Default|GetLastKnownPlayerCoor)))))
    (bind _output_get (Variables|Default|SetLastKnownPlayerCoor (Utilities|GetChunkCoordinates)))
    (if (not (Utilities|Array|ContainsItem (Variables|Default|GetGrid) _output_get))
      (CallFunction|SpawnNewChunksWithinRenderRange)
      (Utilities|Array|AddUnique (Variables|Default|GetGrid) _output_get))))

(fn ConstructionScript)

(fn SpawnNewChunksWithinRenderRange
  (bind _coordinates (Utilities|GetChunkCoordinates))
  (bind _renderrange (Variables|Default|GetRenderRange))
  (bind _renderrange_2 (Variables|Default|GetRenderRange))
  (bind _chunksize (Variables|Default|GetChunkSize))
  (for _index (range (* _renderrange_2 -1) _renderrange_2)
    (LocalVariables|SetTMP_X _index)
    (for _index_2 (range (* _renderrange -1) _renderrange)
      (LocalVariables|SetTMP_Y _index_2)
      (Components|InstancedStaticMesh|AddInstance (Variables|Default|GetInstancedStaticMesh) (Math|Conversions|ToTransform(Vector) (Math|Vector|MakeVector (Math|Conversions|ToFloat(Integer) (* (+ (.x _coordinates) (LocalVariables|GetTMP_X)) _chunksize)) (Math|Conversions|ToFloat(Integer) (* (+ (.y _coordinates) (LocalVariables|GetTMP_Y)) _chunksize)) 0.0)) false))))