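; World generator actor that spawns BP_WFC_ChunkGeneration chunks around the player as they cross chunk boundaries.
; Each missing chunk within RenderRange receives border cells from its four generated neighbours as InputGrid, so wave function collapse can match edges.
; After spawning, it busy-waits on IsGenerated before registering the chunk, and never removes chunks.
; CreateTileSet builds tile adjacency from matching sides but is not called here.
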(event Custom|PlayerHasChangedChankPos
  (bind _intpoint (Utilities|GetPlayerPos))
  (bind _renderrange (Variables|Default|GetRenderRange))
  (bind _renderrange_2 (Variables|Default|GetRenderRange))
  (bind _chunksize (Variables|Default|GetChunkSize))
  (for _index (range (* _renderrange_2 -1) _renderrange_2)
    (Variables|Default|SetTMP_Y _index)
    (for _index_2 (range (* _renderrange -1) _renderrange)
      (Variables|Default|SetTMP_X _index_2)
      (bind _output_get (Variables|Default|SetChunkPos (Utilities|Struct|MakeIntPoint (+ (.x _intpoint) (Variables|Default|GetTMP_X)) (+ (.y _intpoint) (Variables|Default|GetTMP_Y)))))
      (if (not (Utilities|Array|ContainsItem (Variables|Default|GetChunkGridPos) _output_get))
        (Utilities|FlowControl|Sequence
          (:then_0
            (Utilities|Array|Clear (Variables|Default|GetNeighbourGrid))
            (Utilities|FlowControl|Sequence
              (:then_0
                (bind (_array_element _error) (CallFunction|FindChunkbyPos (Utilities|Struct|MakeIntPoint (.x (Variables|Default|GetChunkPos)) (- (.y (Variables|Default|GetChunkPos)) 1))))
                (if (not _error)
                  (if (Variables|/Game/Blueprints/ProceduralGeneration/Blueprints/ChunkBasedGeneration/BP_WFC_ChunkGeneration.BP_WFC_ChunkGeneration_C|GetIsGenerated (.Chunk (Utilities|Struct|BreakBP_Chunk _array_element)))
                    (for _index_3 (range 0 (- (.x (Variables|Default|GetChunkIntPointSize)) 1))
                      (bind (_array_element_2 _error_2) (CallFunction|FindCellbyPos (Variables|/Game/Blueprints/ProceduralGeneration/Blueprints/ChunkBasedGeneration/BP_WFC_ChunkGeneration.BP_WFC_ChunkGeneration_C|GetGrid (.Chunk (Utilities|Struct|BreakBP_Chunk _array_element))) (Utilities|Struct|MakeIntPoint _index_3 (- (.y (Variables|Default|GetChunkIntPointSize)) 1))))
                      (if (not _error_2)
                        (Utilities|Array|AddUnique (Variables|Default|GetNeighbourGrid) (Utilities|Struct|MakeBP_Cell true (.Options (Utilities|Struct|BreakBP_Cell _array_element_2)) (Utilities|Struct|MakeIntPoint (.x (.Position (Utilities|Struct|BreakBP_Cell _array_element_2))) -1) 0)))))))
              (:then_1
                (bind (_array_element_3 _error_3) (CallFunction|FindChunkbyPos (Utilities|Struct|MakeIntPoint (+ (.x (Variables|Default|GetChunkPos)) 1) (.y (Variables|Default|GetChunkPos)))))
                (if (not _error_3)
                  (if (Variables|/Game/Blueprints/ProceduralGeneration/Blueprints/ChunkBasedGeneration/BP_WFC_ChunkGeneration.BP_WFC_ChunkGeneration_C|GetIsGenerated (.Chunk (Utilities|Struct|BreakBP_Chunk _array_element_3)))
                    (for _index_4 (range 0 (- (.y (Variables|Default|GetChunkIntPointSize)) 1))
                      (bind (_array_element_4 _error_4) (CallFunction|FindCellbyPos (Variables|/Game/Blueprints/ProceduralGeneration/Blueprints/ChunkBasedGeneration/BP_WFC_ChunkGeneration.BP_WFC_ChunkGeneration_C|GetGrid (.Chunk (Utilities|Struct|BreakBP_Chunk _array_element_3))) (Utilities|Struct|MakeIntPoint 0 _index_4)))
                      (if (not _error_4)
                        (Utilities|Array|AddUnique (Variables|Default|GetNeighbourGrid) (Utilities|Struct|MakeBP_Cell true (.Options (Utilities|Struct|BreakBP_Cell _array_element_4)) (Utilities|Struct|MakeIntPoint (.x (Variables|Default|GetChunkIntPointSize)) (.y (.Position (Utilities|Struct|BreakBP_Cell _array_element_4)))) 0)))))))
              (:then_2
                (bind (_array_element_5 _error_5) (CallFunction|FindChunkbyPos (Utilities|Struct|MakeIntPoint (.x (Variables|Default|GetChunkPos)) (+ (.y (Variables|Default|GetChunkPos)) 1))))
                (if (not _error_5)
                  (if (Variables|/Game/Blueprints/ProceduralGeneration/Blueprints/ChunkBasedGeneration/BP_WFC_ChunkGeneration.BP_WFC_ChunkGeneration_C|GetIsGenerated (.Chunk (Utilities|Struct|BreakBP_Chunk _array_element_5)))
                    (for _index_5 (range 0 (- (.x (Variables|Default|GetChunkIntPointSize)) 1))
                      (bind (_array_element_6 _error_6) (CallFunction|FindCellbyPos (Variables|/Game/Blueprints/ProceduralGeneration/Blueprints/ChunkBasedGeneration/BP_WFC_ChunkGeneration.BP_WFC_ChunkGeneration_C|GetGrid (.Chunk (Utilities|Struct|BreakBP_Chunk _array_element_5))) (Utilities|Struct|MakeIntPoint _index_5 0)))
                      (if (not _error_6)
                        (Utilities|Array|AddUnique (Variables|Default|GetNeighbourGrid) (Utilities|Struct|MakeBP_Cell true (.Options (Utilities|Struct|BreakBP_Cell _array_element_6)) (Utilities|Struct|MakeIntPoint (.x (.Position (Utilities|Struct|BreakBP_Cell _array_element_6))) (.y (Variables|Default|GetChunkIntPointSize))) 0)))))))
              (:then_3
                (bind (_array_element_7 _error_7) (CallFunction|FindChunkbyPos (Utilities|Struct|MakeIntPoint (- (.x (Variables|Default|GetChunkPos)) 1) (.y (Variables|Default|GetChunkPos)))))
                (if (not _error_7)
                  (if (Variables|/Game/Blueprints/ProceduralGeneration/Blueprints/ChunkBasedGeneration/BP_WFC_ChunkGeneration.BP_WFC_ChunkGeneration_C|GetIsGenerated (.Chunk (Utilities|Struct|BreakBP_Chunk _array_element_7)))
                    (for _index_6 (range 0 (- (.y (Variables|Default|GetChunkIntPointSize)) 1))
                      (bind (_array_element_8 _error_8) (CallFunction|FindCellbyPos (Variables|/Game/Blueprints/ProceduralGeneration/Blueprints/ChunkBasedGeneration/BP_WFC_ChunkGeneration.BP_WFC_ChunkGeneration_C|GetGrid (.Chunk (Utilities|Struct|BreakBP_Chunk _array_element_7))) (Utilities|Struct|MakeIntPoint (- (.x (Variables|Default|GetChunkIntPointSize)) 1) _index_6)))
                      (if (not _error_8)
                        (Utilities|Array|AddUnique (Variables|Default|GetNeighbourGrid) (Utilities|Struct|MakeBP_Cell true (.Options (Utilities|Struct|BreakBP_Cell _array_element_8)) (Utilities|Struct|MakeIntPoint -1 (.y (.Position (Utilities|Struct|BreakBP_Cell _array_element_8)))) 0)))))))
              (:then_4)))
          (:then_1
            (Development|PrintString (Utilities|String|ToString(Integer) (Variables|Default|GetChunkPos)))
            (bind _returnvalue (Game|SpawnActorfromClass "/Game/Blueprints/ProceduralGeneration/Blueprints/ChunkBasedGeneration/BP_WFC_ChunkGeneration.BP_WFC_ChunkGeneration_C" (Math|Transform|MakeTransform (Math|Vector|MakeVector (* (.x (Variables|Default|GetChunkPos)) _chunksize) (* (.y (Variables|Default|GetChunkPos)) _chunksize) 0.0) "0, 0, 0" (.scale (Transformation|GetActorTransform))) "Undefined" 0 (Variables|Default|GetTile%20Size) (Math|Random|MakeRandomStream (Utilities|RandomSeed)) (Variables|Default|GetTileset_I) (Variables|Default|GetChunkIntPointSize) (Variables|Default|GetNeighbourGrid) 0))
            (Utilities|FlowControl|Sequence
              (:then_0
                (CallFunction|Wait _returnvalue))
              (:then_1
                (Utilities|Array|AddUnique (Variables|Default|GetChunkGridPos) (Variables|Default|GetChunkPos))
                (Utilities|Array|AddUnique (Variables|Default|GetChunkGrid) (Utilities|Struct|MakeBP_Chunk (Variables|Default|GetChunkPos) _returnvalue))))))))))

(event EventBeginPlay
  (CallFunction|PlayerHasChangedChankPos))

(event EventTick
  (params (DeltaSeconds :type Float%20%28single-precision%29))
  (bind _intpoint (Utilities|GetPlayerPos))
  (if (not (and (== (.x _intpoint) (.x (Variables|Default|GetLastKnownPlayerChankPos))) (== (.y _intpoint) (.y (Variables|Default|GetLastKnownPlayerChankPos)))))
    (bind _output_get (Variables|Default|SetLastKnownPlayerChankPos (Utilities|GetPlayerPos)))
    (CallFunction|PlayerHasChangedChankPos)
    (Development|PrintString (Utilities|String|ToString(Integer) _output_get))))

(fn ConstructionScript)

(fn FindChunkbyPos
  (params (Pos :type Int%20Point%20Structure))
  (bind (_x _y) (Utilities|Struct|BreakIntPoint Pos))
  (for _array_element (Variables|Default|GetChunkGrid)
    (if (and (== (.X (Utilities|Struct|BreakIntPoint (.Position (Utilities|Struct|BreakBP_Chunk _array_element)))) _x) (== (.Y (Utilities|Struct|BreakIntPoint (.Position (Utilities|Struct|BreakBP_Chunk _array_element)))) _y))
      (return _array_element false)))
  (return "" true))

(fn Wait
  (params (Chunk :type BP%20WFC%20Chunk%20Generation%20Object%20Reference))
  (while (not (Variables|/Game/Blueprints/ProceduralGeneration/Blueprints/ChunkBasedGeneration/BP_WFC_ChunkGeneration.BP_WFC_ChunkGeneration_C|GetIsGenerated Chunk))
    _))

(fn FindCellbyPos
  (params (Grid :type Array%20of%20BP%20Cell%20Structures) (Pos :type Int%20Point%20Structure))
  (bind (_x _y) (Utilities|Struct|BreakIntPoint Pos))
  (for _array_element Grid
    (if (and (== (.X (Utilities|Struct|BreakIntPoint (.Position (Utilities|Struct|BreakBP_Cell _array_element)))) _x) (== (.Y (Utilities|Struct|BreakIntPoint (.Position (Utilities|Struct|BreakBP_Cell _array_element)))) _y))
      (return _array_element false)))
  (return "" true))

(fn CreateTileSet
  (Variables|Default|SetTileset (Variables|Default|GetTileset_I))
  (for _array_element (Variables|/Game/Blueprints/ProceduralGeneration/Structures/Side/BP_TileSet.BP_TileSet_C|GetTiles (Variables|Default|GetTileset))
    (for _array_element_2 (Variables|/Game/Blueprints/ProceduralGeneration/Structures/Side/BP_TileSet.BP_TileSet_C|GetTiles (Variables|Default|GetTileset))
      (Utilities|FlowControl|Sequence
        (:then_0
          (if (Utilities|Enum|Equal(Enum) (Variables|/Game/Blueprints/ProceduralGeneration/Structures/BP_Tile.BP_Tile_C|GetSIDE_UP _array_element) (Variables|/Game/Blueprints/ProceduralGeneration/Structures/BP_Tile.BP_Tile_C|GetSIDE_DOWN _array_element_2))
            (Utilities|Array|AddUnique (Variables|/Game/Blueprints/ProceduralGeneration/Structures/BP_Tile.BP_Tile_C|GetUP _array_element) _array_element_2)))
        (:then_1
          (if (Utilities|Enum|Equal(Enum) (Variables|/Game/Blueprints/ProceduralGeneration/Structures/BP_Tile.BP_Tile_C|GetSIDE_RIGHT _array_element) (Variables|/Game/Blueprints/ProceduralGeneration/Structures/BP_Tile.BP_Tile_C|GetSIDE_LEFT _array_element_2))
            (Utilities|Array|AddUnique (Variables|/Game/Blueprints/ProceduralGeneration/Structures/BP_Tile.BP_Tile_C|GetRIGHT _array_element) _array_element_2)))
        (:then_2
          (if (Utilities|Enum|Equal(Enum) (Variables|/Game/Blueprints/ProceduralGeneration/Structures/BP_Tile.BP_Tile_C|GetSIDE_DOWN _array_element) (Variables|/Game/Blueprints/ProceduralGeneration/Structures/BP_Tile.BP_Tile_C|GetSIDE_UP _array_element_2))
            (Utilities|Array|AddUnique (Variables|/Game/Blueprints/ProceduralGeneration/Structures/BP_Tile.BP_Tile_C|GetDOWN _array_element) _array_element_2)))
        (:then_3
          (if (Utilities|Enum|Equal(Enum) (Variables|/Game/Blueprints/ProceduralGeneration/Structures/BP_Tile.BP_Tile_C|GetSIDE_LEFT _array_element) (Variables|/Game/Blueprints/ProceduralGeneration/Structures/BP_Tile.BP_Tile_C|GetSIDE_RIGHT _array_element_2))
            (Utilities|Array|AddUnique (Variables|/Game/Blueprints/ProceduralGeneration/Structures/BP_Tile.BP_Tile_C|GetLEFT _array_element) _array_element_2)))))))