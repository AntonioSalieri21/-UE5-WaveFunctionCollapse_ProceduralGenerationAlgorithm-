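; Actor that procedurally builds a tile room with Wave Function Collapse on BeginPlay or a dev input action.
; CreateTileSet derives each tile's allowed neighbours from matching side values, and CreateGrid fills a RoomSize grid with every tile option.
; Each step narrows options from four neighbours, then collapses the first lowest-entropy cell to a random tile.
; Collapsed cells are redrawn as instanced meshes every step until completion or contradiction.
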(event EventBeginPlay
  (CallFunction|Clear)
  (CallFunction|StartGeneration)
  (Development|PrintString (Utilities|String|ToString(Float) (- (.PartialSeconds (Class|GameplayStatics|GetAccurateRealTime)) (Variables|Default|GetGenerationTime))))
  (Variables|Default|SetGenerationTime (- (.PartialSeconds (Class|GameplayStatics|GetAccurateRealTime)) (Variables|Default|GetGenerationTime))))

(event Collision|EventActorBeginOverlap
  (params (OtherActor :type Actor%20Object%20Reference)))

(event EventTick
  (params (DeltaSeconds :type Float%20%28single-precision%29)))

(event Input|ActionEvents|InputActionMapGeneration(DEVELOP)
  (params (Key :type Key%20Structure :default "None"))
  (:Pressed
    (CallFunction|Clear :!label _label)
    (CallFunction|StartGeneration)
    (Development|PrintString (Utilities|String|ToString(Float) (- (.PartialSeconds (Class|GameplayStatics|GetAccurateRealTime)) (Variables|Default|GetGenerationTime))))
    (Variables|Default|SetGenerationTime (- (.PartialSeconds (Class|GameplayStatics|GetAccurateRealTime)) (Variables|Default|GetGenerationTime))))
  (:Released
    (goto _label)))

(fn ConstructionScript)

(fn StartGeneration
  (CallFunction|CreateTileSet)
  (Utilities|Array|Clear (Variables|Default|GetGrid))
  (CallFunction|CreateGrid)
  ;[1 1 1] RandomStartElementCollapse
  (CallFunction|CollapseCell)
  (CallFunction|Draw)
  (while (not (Variables|Default|GetIsCollapsed))
    (CallFunction|OneGenerationStep)
    (bind (_iscollapsed _arraylength _iserror) (CallFunction|IsGridCollapsed (Variables|Default|GetGrid)))
    (if _iserror
      (Variables|Default|SetIsCollapsed true)
      (Development|PrintString "ERROR OF GENERATION")
      (else
        (Variables|Default|SetIsCollapsed _iscollapsed)))))

(fn CreateGrid
  (for _index (range 0 (- (.y (Variables|Default|GetRoomSize)) 1))
    (for _index_2 (range 0 (- (.x (Variables|Default|GetRoomSize)) 1))
      (Utilities|Array|Add (Variables|Default|GetGrid) (Utilities|Struct|MakeBP_Cell false (Variables|/Game/Blueprints/ProceduralGeneration/Structures/Side/BP_TileSet.BP_TileSet_C|GetTiles (Variables|Default|GetTileset)) (Utilities|Struct|MakeIntPoint _index_2 _index) 0)))))

(fn Draw
  (bind _tilesize (Variables|Default|GetTileSize))
  (CallFunction|Clear)
  (for _array_element (Variables|Default|GetGrid)
    (bind _output_get (LocalVariables|SetCell _array_element))
    (if (.collapsed _output_get)
      (bind _returnvalue (AddComponent|AddInstancedStaticMeshComponent false))
      (Components|StaticMesh|SetStaticMesh _returnvalue (Variables|/Game/Blueprints/ProceduralGeneration/Structures/BP_Tile.BP_Tile_C|GetStatic%20Mesh (Utilities|Array|Get(acopy) (.options _output_get))))
      (Components|InstancedStaticMesh|AddInstance _returnvalue (Math|Transform|MakeTransform (Math|Vector|MakeVector (Math|Conversions|ToFloat(Integer) (* (.X (Utilities|Struct|BreakIntPoint (.position _output_get))) _tilesize)) (Math|Conversions|ToFloat(Integer) (* (.Y (Utilities|Struct|BreakIntPoint (.position _output_get))) _tilesize)) 0.0) (Math|Rotator|MakeRotator 0.0 0.0 (.yaw (Variables|/Game/Blueprints/ProceduralGeneration/Structures/BP_Tile.BP_Tile_C|GetRotation (Utilities|Array|Get(acopy) (.options _output_get))))) "1.000000,1.000000,1.000000") false)
      (Utilities|Array|Add (Variables|Default|GetISM) _returnvalue))))

(fn CollapseCell
  (bind _exitarray1 (CallFunction|RemoveCollapsedCells))
  (bind _output_get (LocalVariables|SetGridCopy _exitarray1))
  (CallFunction|CollapseRandomLeastEnthropyCell _output_get))

(fn RemoveCollapsedCells
  (bind _output_get (LocalVariables|SetGridCopy (Variables|Default|GetGrid)))
  (for _array_element _output_get
    (if (not (.Collapsed (Utilities|Struct|BreakBP_Cell _array_element)))
      (Utilities|Array|Add (LocalVariables|GetExitArray) _array_element)))
  (return (LocalVariables|GetExitArray)))

(fn CollapseRandomLeastEnthropyCell
  (params (GridCopy :type Array%20of%20BP%20Cell%20Structures))
  (Utilities|FlowControl|Sequence
    (:then_0
      (LocalVariables|Setlen (Utilities|Array|Length (.options (Utilities|Array|Get(acopy) GridCopy))))
      (for _array_element GridCopy
        (if (and (not (.collapsed _array_element)) (< (Utilities|Array|Length (.options _array_element)) (LocalVariables|Getlen)))
          (LocalVariables|Setlen (Utilities|Array|Length (.options _array_element))))))
    (:then_1
      (bind (_array_element_2 _array_index) (Utilities|Array|ForEachLoopwithBreak (Variables|Default|GetGrid) :!label _label)
        (:LoopBody
          (if (and (<= (Utilities|Array|Length (.Options (Utilities|Struct|BreakBP_Cell _array_element_2))) (LocalVariables|Getlen)) (not (.Collapsed (Utilities|Struct|BreakBP_Cell _array_element_2))))
            (Utilities|Array|SetArrayElem (Variables|Default|GetGrid) _array_index (Utilities|Struct|MakeBP_Cell true (Utilities|Array|MakeArray (.Element (Utilities|RandomElementOfArray (.Options (Utilities|Struct|BreakBP_Cell _array_element_2))))) (.Position (Utilities|Struct|BreakBP_Cell _array_element_2)) 0))
            (goto _label Break)))))
    (:then_2
      (Development|PrintString "-------------------------")
      (Development|PrintString "Cleaned array:")
      (for _array_element_3 GridCopy
        (Development|PrintString (Utilities|String|ToString(Integer) (Utilities|Array|Length (.Options (Utilities|Struct|BreakBP_Cell _array_element_3)))))))))

(fn Clear
  (for _array_element (Variables|Default|GetISM)
    (Components|InstancedStaticMesh|ClearInstances _array_element))
  (Utilities|Array|Clear (Variables|Default|GetISM))
  (Variables|Default|SetIsCollapsed false))

(fn OneGenerationStep
  (CallFunction|UpdateEnthropy)
  (CallFunction|CollapseCell)
  (CallFunction|Draw))

(fn UpdateEnthropy
  (LocalVariables|SetnextGrid (Variables|Default|GetGrid))
  (for (_array_element _array_index) (Variables|Default|GetGrid)
    (LocalVariables|SetIndex _array_index)
    (if (.Collapsed (Utilities|Struct|BreakBP_Cell _array_element))
      (Utilities|Array|SetArrayElem (LocalVariables|GetnextGrid) _array_index _array_element)
      (else
        (LocalVariables|SetCurrentCell _array_element)
        (LocalVariables|SetOptions (Variables|/Game/Blueprints/ProceduralGeneration/Structures/Side/BP_TileSet.BP_TileSet_C|GetTiles (Variables|Default|GetTileset)))
        (Utilities|FlowControl|Sequence
          (:then_0
            (bind (_array_element_2 _error) (CallFunction|GetArrayElembyPos (Variables|Default|GetGrid) (LocalVariables|GetCurrentCell) (Utilities|Struct|MakeIntPoint 0 -1)))
            (if (not _error)
              (bind _output_get (LocalVariables|SetNeighbour _array_element_2))
              (Utilities|Array|Clear (LocalVariables|GetvalidOptions))
              (for _array_element_3 (.Options (Utilities|Struct|BreakBP_Cell _output_get))
                (bind _output_get_2 (LocalVariables|Setvalid (Variables|/Game/Blueprints/ProceduralGeneration/Structures/BP_Tile.BP_Tile_C|GetUP _array_element_3)))
                (for _array_element_4 _output_get_2
                  (Utilities|Array|AddUnique (LocalVariables|GetvalidOptions) _array_element_4)))
              (bind _options1 (CallFunction|CheckValid (LocalVariables|GetOptions) (LocalVariables|GetvalidOptions)))
              (LocalVariables|SetOptions _options1)))
          (:then_1
            (bind (_array_element_5 _error_2) (CallFunction|GetArrayElembyPos (Variables|Default|GetGrid) (LocalVariables|GetCurrentCell) (Utilities|Struct|MakeIntPoint 1 0)))
            (if (not _error_2)
              (bind _output_get_3 (LocalVariables|SetNeighbour _array_element_5))
              (Utilities|Array|Clear (LocalVariables|GetvalidOptions))
              (for _array_element_6 (.Options (Utilities|Struct|BreakBP_Cell _output_get_3))
                (bind _output_get_4 (LocalVariables|Setvalid (Variables|/Game/Blueprints/ProceduralGeneration/Structures/BP_Tile.BP_Tile_C|GetRIGHT _array_element_6)))
                (for _array_element_7 _output_get_4
                  (Utilities|Array|AddUnique (LocalVariables|GetvalidOptions) _array_element_7)))
              (bind _options1_2 (CallFunction|CheckValid (LocalVariables|GetOptions) (LocalVariables|GetvalidOptions)))
              (LocalVariables|SetOptions _options1_2)))
          (:then_2
            (bind (_array_element_8 _error_3) (CallFunction|GetArrayElembyPos (Variables|Default|GetGrid) (LocalVariables|GetCurrentCell) (Utilities|Struct|MakeIntPoint 0 1)))
            (if (not _error_3)
              (bind _output_get_5 (LocalVariables|SetNeighbour _array_element_8))
              (Utilities|Array|Clear (LocalVariables|GetvalidOptions))
              (for _array_element_9 (.Options (Utilities|Struct|BreakBP_Cell _output_get_5))
                (bind _output_get_6 (LocalVariables|Setvalid (Variables|/Game/Blueprints/ProceduralGeneration/Structures/BP_Tile.BP_Tile_C|GetDOWN _array_element_9)))
                (for _array_element_10 _output_get_6
                  (Utilities|Array|AddUnique (LocalVariables|GetvalidOptions) _array_element_10)))
              (bind _options1_3 (CallFunction|CheckValid (LocalVariables|GetOptions) (LocalVariables|GetvalidOptions)))
              (LocalVariables|SetOptions _options1_3)))
          (:then_3
            (bind (_array_element_11 _error_4) (CallFunction|GetArrayElembyPos (Variables|Default|GetGrid) (LocalVariables|GetCurrentCell) (Utilities|Struct|MakeIntPoint -1 0)))
            (if (not _error_4)
              (bind _output_get_7 (LocalVariables|SetNeighbour _array_element_11))
              (Utilities|Array|Clear (LocalVariables|GetvalidOptions))
              (for _array_element_12 (.Options (Utilities|Struct|BreakBP_Cell _output_get_7))
                (bind _output_get_8 (LocalVariables|Setvalid (Variables|/Game/Blueprints/ProceduralGeneration/Structures/BP_Tile.BP_Tile_C|GetLEFT _array_element_12)))
                (for _array_element_13 _output_get_8
                  (Utilities|Array|AddUnique (LocalVariables|GetvalidOptions) _array_element_13)))
              (bind _options1_4 (CallFunction|CheckValid (LocalVariables|GetOptions) (LocalVariables|GetvalidOptions)))
              (LocalVariables|SetOptions _options1_4)))
          (:then_4
            (Utilities|Array|SetArrayElem (LocalVariables|GetnextGrid) (LocalVariables|GetIndex) (Utilities|Struct|MakeBP_Cell false (LocalVariables|GetOptions) (.position (LocalVariables|GetCurrentCell)) 0)))))))
  (Variables|Default|SetGrid (LocalVariables|GetnextGrid)))

(fn IsGridCollapsed
  (params (Grid :type Array%20of%20BP%20Cell%20Structures))
  (for _array_element Grid
    (if (not (< (Utilities|Array|Length (.Options (Utilities|Struct|BreakBP_Cell _array_element))) 1))
      (if (.Collapsed (Utilities|Struct|BreakBP_Cell _array_element))
        _
        (else
          (LocalVariables|SetIsGridCollapsed false)))
      (Math|Integer|IncrementInt (LocalVariables|GetLength))
      (else
        (return (LocalVariables|GetIsGridCollapsed) (LocalVariables|GetLength) true))))
  (return (LocalVariables|GetIsGridCollapsed) (LocalVariables|GetLength) false))

(fn CheckValid
  (params (options :type Array%20of%20BP%20Tile%20Object%20References) (validOptions :type Array%20of%20BP%20Tile%20Object%20References))
  (LocalVariables|SetTMP_Options options)
  (LocalVariables|SetTMP_ValidOptions validOptions)
  (for _array_element options
    (if (not (Utilities|Array|ContainsItem (LocalVariables|GetTMP_ValidOptions) _array_element))
      (Utilities|Array|RemoveItem (LocalVariables|GetTMP_Options) _array_element)))
  (return (LocalVariables|GetTMP_Options)))

(fn CreateTileSet
  (Variables|Default|SetTileset (Variables|Default|GetTileset_I))
  (for _array_element (Variables|/Game/Blueprints/ProceduralGeneration/Structures/Side/BP_TileSet.BP_TileSet_C|GetTiles (Variables|Default|GetTileset))
    (for _array_element_2 (Variables|/Game/Blueprints/ProceduralGeneration/Structures/Side/BP_TileSet.BP_TileSet_C|GetTiles (Variables|Default|GetTileset))
      (Utilities|FlowControl|Sequence
        (:then_0
          (if (Utilities|Enum|Equal(Enum) (Variables|/Game/Blueprints/ProceduralGeneration/Structures/BP_Tile.BP_Tile_C|GetSIDE_UP _array_element) (Variables|/Game/Blueprints/ProceduralGeneration/Structures/BP_Tile.BP_Tile_C|GetSIDE_DOWN _array_element_2))
            (Utilities|Array|AddUnique (Variables|/Game/Blueprints/ProceduralGeneration/Structures/BP_Tile.BP_Tile_C|GetUP _array_element) _array_element_2)))
        (:then_1
          (if (Utilities|Enum|Equal(Enum) (Variables|/Game/Blueprints/ProceduralGeneration/Structures/BP_Tile.BP_Tile_C|GetSIDE_RIGHT _array_element) (Variables|/Game/Blueprints/ProceduralGeneration/Structures/BP_Tile.BP_Tile_C|GetSIDE_LEFT _array_element_2))
            (Utilities|Array|AddUnique (Variables|/Game/Blueprints/ProceduralGeneration/Structures/BP_Tile.BP_Tile_C|GetRIGHT _array_element) _array_element_2)))
        (:then_2
          (if (Utilities|Enum|Equal(Enum) (Variables|/Game/Blueprints/ProceduralGeneration/Structures/BP_Tile.BP_Tile_C|GetSIDE_DOWN _array_element) (Variables|/Game/Blueprints/ProceduralGeneration/Structures/BP_Tile.BP_Tile_C|GetSIDE_UP _array_element_2))
            (Utilities|Array|AddUnique (Variables|/Game/Blueprints/ProceduralGeneration/Structures/BP_Tile.BP_Tile_C|GetDOWN _array_element) _array_element_2)))
        (:then_3
          (if (Utilities|Enum|Equal(Enum) (Variables|/Game/Blueprints/ProceduralGeneration/Structures/BP_Tile.BP_Tile_C|GetSIDE_LEFT _array_element) (Variables|/Game/Blueprints/ProceduralGeneration/Structures/BP_Tile.BP_Tile_C|GetSIDE_RIGHT _array_element_2))
            (Utilities|Array|AddUnique (Variables|/Game/Blueprints/ProceduralGeneration/Structures/BP_Tile.BP_Tile_C|GetLEFT _array_element) _array_element_2)))))))

(fn GridInfo
  (for (_array_element _array_index) (Variables|Default|GetGrid)
    (Development|PrintString "----------")
    (Development|PrintString (Utilities|String|ToString(Integer) _array_index))
    (Development|PrintString "Tile:")
    (Development|PrintString (Utilities|GetDisplayName (Utilities|Array|Get(acopy) (.Options (Utilities|Struct|BreakBP_Cell _array_element)))))))

(fn GetArrayElembyPos
  (params (Grid :type Array%20of%20BP%20Cell%20Structures) (CurrentCell :type BP%20Cell%20Structure) (NeighbourBias :type Int%20Point%20Structure))
  (bind _position (Utilities|Struct|BreakBP_Cell CurrentCell))
  (bind (_x _y) (Utilities|Struct|BreakIntPoint NeighbourBias))
  (bind (_x_2 _y_2) (Utilities|Struct|BreakIntPoint _position))
  (LocalVariables|SetTargetPos (Utilities|Struct|MakeIntPoint (+ _x_2 _x) (+ _y_2 _y)))
  (bind _array_element (Utilities|Array|ForEachLoopwithBreak Grid)
    (:LoopBody
      (if (and (== (.X (Utilities|Struct|BreakIntPoint (.Position (Utilities|Struct|BreakBP_Cell _array_element)))) (.x (LocalVariables|GetTargetPos))) (== (.Y (Utilities|Struct|BreakIntPoint (.Position (Utilities|Struct|BreakBP_Cell _array_element)))) (.y (LocalVariables|GetTargetPos))))
        (return _array_element false)))
    (:Completed
      (return "" true))))