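; BP_WFC_Start generates a DIM×DIM tile map with Wave Function Collapse, though nothing live in this file calls StartGeneration.
; CreateGrid gives every cell all Tileset tiles, then CollapseCell fixes a random tile in a random lowest-option cell.
; Each step, UpdateEnthropy narrows options from four neighbours' adjacency lists, then collapses again, without backtracking.
; Draw rebuilds collapsed tiles as one instanced static mesh component per cell after every step.
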(event EventBeginPlay)

(event Collision|EventActorBeginOverlap
  (params (OtherActor :type Actor%20Object%20Reference)))

(event EventTick
  (params (DeltaSeconds :type Float%20%28single-precision%29)))

(fn ConstructionScript)

(fn StartGeneration
  (Utilities|Array|Clear (Variables|Default|GetGrid))
  (CallFunction|CreateGrid)
  ;[1 1 1] RandomStartElementCollapse
  (CallFunction|CollapseCell)
  (CallFunction|Draw)
  (while (not (LocalVariables|GetIsCollapsed))
    (CallFunction|OneGenerationStep)
    (bind _iscollapsed (CallFunction|IsGridCollapsed (Variables|Default|GetGrid)))
    (LocalVariables|SetIsCollapsed _iscollapsed)))

(fn CreateGrid
  (bind _dim (Variables|Default|GetDIM))
  (for _index (range 0 (- (* _dim _dim) 1))
    (Utilities|Array|Add (Variables|Default|GetGrid) (Utilities|Struct|MakeBP_Cell false (Variables|/Game/Blueprints/ProceduralGeneration/Structures/Side/BP_TileSet.BP_TileSet_C|GetTiles (Variables|Default|GetTileset)) "(X=0,Y=0)" _index))))

(fn Draw
  (CallFunction|Clear)
  (for _index (range 0 (- (Variables|Default|GetDIM) 1))
    (LocalVariables|SetJ _index)
    (for _index_2 (range 0 (- (Variables|Default|GetDIM) 1))
      (LocalVariables|SetI _index_2)
      (bind _output_get (LocalVariables|SetIndex (+ (LocalVariables|GetI) (* (LocalVariables|GetJ) (Variables|Default|GetDIM)))))
      (bind _output_get_2 (LocalVariables|SetCell (Utilities|Array|Get(acopy) (Variables|Default|GetGrid) _output_get)))
      (if (.collapsed _output_get_2)
        (bind _returnvalue (AddComponent|AddInstancedStaticMeshComponent false))
        (Components|StaticMesh|SetStaticMesh _returnvalue (Variables|/Game/Blueprints/ProceduralGeneration/Structures/BP_Tile.BP_Tile_C|GetStatic%20Mesh (Utilities|Array|Get(acopy) (.options _output_get_2))))
        (Components|InstancedStaticMesh|AddInstance _returnvalue (Math|Transform|MakeTransform (Math|Vector|MakeVector (Math|Conversions|ToFloat(Integer) (* (LocalVariables|GetI) (Variables|Default|GetTileSize))) (Math|Conversions|ToFloat(Integer) (* (LocalVariables|GetJ) (Variables|Default|GetTileSize))) 0.0) (Variables|/Game/Blueprints/ProceduralGeneration/Structures/BP_Tile.BP_Tile_C|GetRotation (Utilities|Array|Get(acopy) (.options _output_get_2))) "1.000000,1.000000,1.000000") false)
        (Utilities|Array|Add (Variables|Default|GetISM) _returnvalue)))))

(fn CollapseCell
  (bind _exitarray1 (CallFunction|SortArraybyEnthropy(BUBBLESORT)))
  (bind _iscollapsed (CallFunction|IsGridCollapsed _exitarray1))
  (if (not _iscollapsed)
    (bind _output_get (LocalVariables|SetGridCopy _exitarray1))
    (CallFunction|CollapseRandomLeastEnthropyCell _output_get)
    (else
      (Development|PrintString "END OF GENERATION"))))

(fn SortArraybyEnthropy(BUBBLESORT)
  (bind _output_get (LocalVariables|SetGridCopy (Variables|Default|GetGrid)))
  (for _array_element _output_get
    (if (not (.Collapsed (Utilities|Struct|BreakBP_Cell _array_element)))
      (Utilities|Array|Add (LocalVariables|GetExitArray) _array_element)))
  (return (LocalVariables|GetExitArray)))

(fn CollapseRandomLeastEnthropyCell
  (params (GridCopy :type Array%20of%20BP%20Cell%20Structures))
  (bind _cleanedarray (LocalVariables|GetCleanedArray))
  (bind _element (Utilities|RandomElementOfArray _cleanedarray))
  (bind (_collapsed _options _position _index) (Utilities|Struct|BreakBP_Cell _element))
  (Utilities|FlowControl|Sequence
    (:then_0
      (Utilities|FlowControl|Sequence
        (:then_0
          (LocalVariables|Setlen (Utilities|Array|Length (.options (Utilities|Array|Get(acopy) GridCopy))))
          (for _array_element GridCopy
            (if (and (not (.collapsed _array_element)) (< (Utilities|Array|Length (.options _array_element)) (LocalVariables|Getlen)))
              (LocalVariables|Setlen (Utilities|Array|Length (.options _array_element))))))
        (:then_1
          (for _array_element_2 GridCopy
            (if (== (Utilities|Array|Length (.Options (Utilities|Struct|BreakBP_Cell _array_element_2))) (LocalVariables|Getlen))
              (Utilities|Array|Add (LocalVariables|GetCleanedArray) _array_element_2))))
        (:then_2
          (Development|PrintString "-------------------------")
          (Development|PrintString "Cleaned array:")
          (for _array_element_3 (LocalVariables|GetCleanedArray)
            (Development|PrintString (Utilities|String|ToString(Integer) (Utilities|Array|Length (.Options (Utilities|Struct|BreakBP_Cell _array_element_3)))))))))
    (:then_1
      (Utilities|Array|SetArrayElem (Variables|Default|GetGrid) _index (Utilities|Struct|MakeBP_Cell true (Utilities|Array|MakeArray (.Element (Utilities|RandomElementOfArray _options))) _position _index)))))

(fn Clear
  (for _array_element (Variables|Default|GetISM)
    (Components|InstancedStaticMesh|ClearInstances _array_element))
  (Utilities|Array|Clear (Variables|Default|GetISM)))

(fn OneGenerationStep
  (CallFunction|UpdateEnthropy)
  (CallFunction|CollapseCell)
  (CallFunction|Draw))

(fn UpdateEnthropy
  (LocalVariables|SetnextGrid (Variables|Default|GetGrid))
  (for _index (range 0 (- (Variables|Default|GetDIM) 1))
    (LocalVariables|Setj _index)
    (for _index_2 (range 0 (- (Variables|Default|GetDIM) 1))
      (LocalVariables|Seti _index_2)
      (bind _output_get (LocalVariables|SetIndex (+ (* (LocalVariables|Getj) (Variables|Default|GetDIM)) (LocalVariables|Geti))))
      (if (.Collapsed (Utilities|Struct|BreakBP_Cell (Utilities|Array|Get(acopy) (Variables|Default|GetGrid) _output_get)))
        (Utilities|Array|SetArrayElem (LocalVariables|GetnextGrid) (LocalVariables|GetIndex) (Utilities|Array|Get(acopy) (Variables|Default|GetGrid) _output_get))
        (else
          (LocalVariables|SetCurrentCell (Utilities|Array|Get(acopy) (Variables|Default|GetGrid) _output_get))
          (LocalVariables|SetOptions (Variables|/Game/Blueprints/ProceduralGeneration/Structures/Side/BP_TileSet.BP_TileSet_C|GetTiles (Variables|Default|GetTileset)))
          (Utilities|FlowControl|Sequence
            (:then_0
              (if (> (LocalVariables|Getj) 0)
                (bind _output_get_2 (LocalVariables|SetNeighbour (Utilities|Array|Get(acopy) (Variables|Default|GetGrid) (+ (* (- (LocalVariables|Getj) 1) (Variables|Default|GetDIM)) (LocalVariables|Geti)))))
                (Utilities|Array|Clear (LocalVariables|GetvalidOptions))
                (for _array_element (.Options (Utilities|Struct|BreakBP_Cell _output_get_2))
                  (bind _output_get_3 (LocalVariables|Setvalid (Variables|/Game/Blueprints/ProceduralGeneration/Structures/BP_Tile.BP_Tile_C|GetUP _array_element)))
                  (for _array_element_2 _output_get_3
                    (Utilities|Array|AddUnique (LocalVariables|GetvalidOptions) _array_element_2)))
                (bind _options1 (CallFunction|CheckValid (LocalVariables|GetOptions) (LocalVariables|GetvalidOptions)))
                (LocalVariables|SetOptions _options1)))
            (:then_1
              (if (< (LocalVariables|Geti) (- (Variables|Default|GetDIM) 1))
                (bind _output_get_4 (LocalVariables|SetNeighbour (Utilities|Array|Get(acopy) (Variables|Default|GetGrid) (+ (* (LocalVariables|Getj) (Variables|Default|GetDIM)) (+ (LocalVariables|Geti) 1)))))
                (Utilities|Array|Clear (LocalVariables|GetvalidOptions))
                (for _array_element_3 (.Options (Utilities|Struct|BreakBP_Cell _output_get_4))
                  (bind _output_get_5 (LocalVariables|Setvalid (Variables|/Game/Blueprints/ProceduralGeneration/Structures/BP_Tile.BP_Tile_C|GetRIGHT _array_element_3)))
                  (for _array_element_4 _output_get_5
                    (Utilities|Array|AddUnique (LocalVariables|GetvalidOptions) _array_element_4)))
                (bind _options1_2 (CallFunction|CheckValid (LocalVariables|GetOptions) (LocalVariables|GetvalidOptions)))
                (LocalVariables|SetOptions _options1_2)))
            (:then_2
              (if (< (LocalVariables|Getj) (- (Variables|Default|GetDIM) 1))
                (bind _output_get_6 (LocalVariables|SetNeighbour (Utilities|Array|Get(acopy) (Variables|Default|GetGrid) (+ (* (+ (LocalVariables|Getj) 1) (Variables|Default|GetDIM)) (LocalVariables|Geti)))))
                (Utilities|Array|Clear (LocalVariables|GetvalidOptions))
                (for _array_element_5 (.Options (Utilities|Struct|BreakBP_Cell _output_get_6))
                  (bind _output_get_7 (LocalVariables|Setvalid (Variables|/Game/Blueprints/ProceduralGeneration/Structures/BP_Tile.BP_Tile_C|GetDOWN _array_element_5)))
                  (for _array_element_6 _output_get_7
                    (Utilities|Array|AddUnique (LocalVariables|GetvalidOptions) _array_element_6)))
                (bind _options1_3 (CallFunction|CheckValid (LocalVariables|GetOptions) (LocalVariables|GetvalidOptions)))
                (LocalVariables|SetOptions _options1_3)))
            (:then_3
              (if (> (LocalVariables|Geti) 0)
                (bind _output_get_8 (LocalVariables|SetNeighbour (Utilities|Array|Get(acopy) (Variables|Default|GetGrid) (+ (* (LocalVariables|Getj) (Variables|Default|GetDIM)) (- (LocalVariables|Geti) 1)))))
                (Utilities|Array|Clear (LocalVariables|GetvalidOptions))
                (for _array_element_7 (.Options (Utilities|Struct|BreakBP_Cell _output_get_8))
                  (bind _output_get_9 (LocalVariables|Setvalid (Variables|/Game/Blueprints/ProceduralGeneration/Structures/BP_Tile.BP_Tile_C|GetLEFT _array_element_7)))
                  (for _array_element_8 _output_get_9
                    (Utilities|Array|AddUnique (LocalVariables|GetvalidOptions) _array_element_8)))
                (bind _options1_4 (CallFunction|CheckValid (LocalVariables|GetOptions) (LocalVariables|GetvalidOptions)))
                (LocalVariables|SetOptions _options1_4)))
            (:then_4
              (Utilities|Array|SetArrayElem (LocalVariables|GetnextGrid) (LocalVariables|GetIndex) (Utilities|Struct|MakeBP_Cell false (LocalVariables|GetOptions) (.position (LocalVariables|GetCurrentCell)) (.index (LocalVariables|GetCurrentCell))))))))))
  (Variables|Default|SetGrid (LocalVariables|GetnextGrid)))

(fn IsGridCollapsed
  (params (Grid :type Array%20of%20BP%20Cell%20Structures))
  (for _array_element Grid
    (if (.Collapsed (Utilities|Struct|BreakBP_Cell _array_element))
      _
      (else
        (LocalVariables|SetIsGridCollapsed false)))
    (Math|Integer|IncrementInt (LocalVariables|GetLength)))
  (return (LocalVariables|GetIsGridCollapsed) (LocalVariables|GetLength)))

(fn CheckValid
  (params (options :type Array%20of%20BP%20Tile%20Object%20References) (validOptions :type Array%20of%20BP%20Tile%20Object%20References))
  (LocalVariables|SetTMP_Options options)
  (LocalVariables|SetTMP_ValidOptions validOptions)
  (for _array_element options
    (if (not (Utilities|Array|ContainsItem (LocalVariables|GetTMP_ValidOptions) _array_element))
      (Utilities|Array|RemoveItem (LocalVariables|GetTMP_Options) _array_element)))
  (return (LocalVariables|GetTMP_Options)))

(fn CreateTileSet
  (for _array_element (Variables|/Game/Blueprints/ProceduralGeneration/Structures/Side/BP_TileSet.BP_TileSet_C|GetTiles (Variables|Default|GetTileset))
    _))