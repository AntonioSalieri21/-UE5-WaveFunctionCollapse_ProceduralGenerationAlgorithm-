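; Generates a tile-based room layout from a TileSet using Wave Function Collapse, starting in both the construction script and BeginPlay.
; GenerateGrid fills RoomSize cells with every tile option and collapses a random one.
; OneStepGeneration runs a single pass: UpdateEnthropy filters options by neighbours' directional adjacency lists, then CollapseCell fixes a lowest-option cell.
; Draw spawns instanced static mesh components for collapsed cells, and cell states print for debugging.
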(event EventBeginPlay
  (CallFunction|StartGeneration))

(event Collision|EventActorBeginOverlap
  (params (OtherActor :type Actor%20Object%20Reference)))

(event EventTick
  (params (DeltaSeconds :type Float%20%28single-precision%29)))

(fn ConstructionScript
  (CallFunction|StartGeneration))

(fn GenerateGrid
  (bind _randomstream (Variables|Default|GetRandomStream))
  (bind _grid (Variables|Default|GetGrid))
  (bind _returnvalue (Utilities|Array|Length _grid))
  (bind _returnvalue_2 (- _returnvalue 1))
  (bind _returnvalue_3 (Math|Random|RandomIntegerinRangefromStream 0 _returnvalue_2 _randomstream))
  (Utilities|FlowControl|Sequence
    (:then_0
      (for _index (range 0 (- (.x (Variables|Default|GetRoomSize)) 1))
        (for _index_2 (range 0 (- (.y (Variables|Default|GetRoomSize)) 1))
          (Utilities|Array|AddUnique (Variables|Default|GetGrid) (Utilities|Struct|MakeBP_Cell false (Variables|/Game/Blueprints/ProceduralGeneration/Structures/Side/BP_TileSet.BP_TileSet_C|GetTiles (Variables|Default|GetTileSet)) "(X=0,Y=0)" 0) _index _index_2))))
    (:then_1
      (bind _output_get (LocalVariables|SetTMP_CELL (Utilities|Array|Get(acopy) _grid _returnvalue_3)))
      (Utilities|Array|SetArrayElem (Variables|Default|GetGrid) _returnvalue_3 (Utilities|Struct|MakeBP_Cell true (Utilities|Array|MakeArray (.Element (Utilities|RandomElementOfArray (Variables|/Game/Blueprints/ProceduralGeneration/Structures/Side/BP_TileSet.BP_TileSet_C|GetTiles (Variables|Default|GetTileSet))))) (.Position (Utilities|Struct|BreakBP_Cell _output_get)))))))

(fn StartGeneration
  (Utilities|Array|Clear (Variables|Default|GetGrid))
  (CallFunction|GenerateGrid)
  (CallFunction|OneStepGeneration))

(fn Draw
  (bind _tilesize (Variables|Default|GetTileSize))
  (CallFunction|Clear)
  (for _index (range 0 (- (.y (Variables|Default|GetRoomSize)) 1))
    (LocalVariables|SetY _index)
    (for _index_2 (range 0 (- (.x (Variables|Default|GetRoomSize)) 1))
      (LocalVariables|SetX _index_2)
      (bind _output_get (LocalVariables|SetIndex (+ (* (LocalVariables|GetY) (.y (Variables|Default|GetRoomSize))) (LocalVariables|GetX))))
      (if (.collapsed (Utilities|Array|Get(acopy) (Variables|Default|GetGrid) _output_get))
        (bind _returnvalue (AddComponent|AddInstancedStaticMeshComponent false))
        (Components|StaticMesh|SetStaticMesh _returnvalue (Variables|/Game/Blueprints/ProceduralGeneration/Structures/BP_Tile.BP_Tile_C|GetStatic%20Mesh (Utilities|Array|Get(acopy) (.options (Utilities|Array|Get(acopy) (Variables|Default|GetGrid) _output_get)))))
        (Components|InstancedStaticMesh|AddInstance _returnvalue (Math|Transform|MakeTransform (Math|Vector|MakeVector (Math|Conversions|ToFloat(Integer) (* (LocalVariables|GetX) _tilesize)) (Math|Conversions|ToFloat(Integer) (* (LocalVariables|GetY) _tilesize)) 0.0) (Variables|/Game/Blueprints/ProceduralGeneration/Structures/BP_Tile.BP_Tile_C|GetRotation (Utilities|Array|Get(acopy) (.options (Utilities|Array|Get(acopy) (Variables|Default|GetGrid) _output_get)))) "1.000000,1.000000,1.000000") false)
        (Utilities|Array|AddUnique (Variables|Default|GetISM) _returnvalue)))))

(fn Clear
  (for _array_element (Variables|Default|GetISM)
    (Class|InstancedStaticMeshComponent|RemoveInstance _array_element))
  (Utilities|Array|Clear (Variables|Default|GetISM))
  (for _array_element_2 (Variables|Default|GetTRC)
    (Components|DestroyComponent _array_element_2))
  (Utilities|Array|Clear (Variables|Default|GetTRC)))

(fn CollapseCell
  (bind _entarray (LocalVariables|GetEntArray))
  (bind (_element _index) (Utilities|RandomElementOfArray _entarray))
  (Utilities|FlowControl|Sequence
    (:then_0
      (for (_array_element _array_index) (Variables|Default|GetGrid)
        (if (> (Utilities|Array|Length (.options _array_element)) 1)
          (Utilities|Array|Add (LocalVariables|GetEntIndexArray) _array_index)
          (Utilities|Array|Add (LocalVariables|GetEntArray) (Utilities|Array|Length (.options _array_element))))))
    (:then_1
      (LocalVariables|SetMinEnt _element)
      (LocalVariables|SetMinCellIndex _index)
      (for (_array_element_2 _array_index_2) (LocalVariables|GetEntArray)
        (if (< _array_element_2 (LocalVariables|GetMinEnt))
          (LocalVariables|SetMinCellIndex _array_index_2)
          (LocalVariables|SetMinEnt _array_element_2))))
    (:then_2
      (bind _output_get (LocalVariables|SetGridPosition (Utilities|Array|Get(acopy) (LocalVariables|GetEntIndexArray) (LocalVariables|GetMinCellIndex))))
      (Utilities|Array|SetArrayElem (Variables|Default|GetGrid) _output_get (Utilities|Struct|MakeBP_Cell true (Utilities|Array|MakeArray (.Element (Utilities|RandomElementOfArray (.options (Utilities|Array|Get(acopy) (Variables|Default|GetGrid) (LocalVariables|GetGridPosition)))))) (.position (Utilities|Array|Get(acopy) (Variables|Default|GetGrid) (LocalVariables|GetGridPosition))))))))

(fn OneStepGeneration
  (CallFunction|UpdateEnthropy)
  (CallFunction|CollapseCell)
  (CallFunction|Draw)
  (for (_array_element _array_index) (Variables|Default|GetGrid)
    (Development|PrintString "------------------------------")
    (Development|PrintText (Utilities|Text|ToText(Integer) _array_index))
    (Development|PrintText (Utilities|Text|ToText(Boolean) (.Collapsed (Utilities|Struct|BreakBP_Cell _array_element))))
    (for _array_element_2 (.Options (Utilities|Struct|BreakBP_Cell _array_element))
      (Development|PrintString (Utilities|GetDisplayName _array_element_2)))
    (Development|PrintString (Utilities|String|ToString(Integer) (.Position (Utilities|Struct|BreakBP_Cell _array_element))))))

(fn UpdateEnthropy
  (LocalVariables|SetTMP_NextGrid (Variables|Default|GetGrid))
  (Utilities|FlowControl|Sequence
    (:then_0
      (for _index (range 0 (- (.y (Variables|Default|GetRoomSize)) 1))
        (LocalVariables|Setj _index)
        (for _index_2 (range 0 (- (.x (Variables|Default|GetRoomSize)) 1))
          (LocalVariables|Seti _index_2)
          (bind _output_get (LocalVariables|SetIndex (+ (* (LocalVariables|Getj) (.y (Variables|Default|GetRoomSize))) (LocalVariables|Geti))))
          (bind _output_get_2 (LocalVariables|SetCurrentCell (Utilities|Array|Get(acopy) (Variables|Default|GetGrid) _output_get)))
          (if (.collapsed _output_get_2)
            (Utilities|Array|SetArrayElem (LocalVariables|GetTMP_NextGrid) (LocalVariables|GetIndex) (LocalVariables|GetCurrentCell))
            (else
              (LocalVariables|SetOptions (.options (LocalVariables|GetCurrentCell)))
              (Utilities|FlowControl|Sequence
                (:then_0
                  (if (> (LocalVariables|Getj) 0)
                    (LocalVariables|SetUp (Utilities|Array|Get(acopy) (Variables|Default|GetGrid) (+ (LocalVariables|Geti) (* (- (LocalVariables|Getj) 1) (.y (Variables|Default|GetRoomSize))))))
                    (Utilities|Array|Clear (LocalVariables|GetvalidOptions))
                    (for _array_element (.options (LocalVariables|GetUp))
                      (bind _output_get_3 (LocalVariables|Setvalid (Variables|/Game/Blueprints/ProceduralGeneration/Structures/BP_Tile.BP_Tile_C|GetUP _array_element)))
                      (for _array_element_2 _output_get_3
                        (Utilities|Array|AddUnique (LocalVariables|GetvalidOptions) _array_element_2))
                      (bind _options1 (CallFunction|CheckValid (LocalVariables|GetOptions) (LocalVariables|GetvalidOptions)))
                      (LocalVariables|SetOptions _options1))))
                (:then_1
                  (if (< (LocalVariables|Geti) (- (.x (Variables|Default|GetRoomSize)) 1))
                    (LocalVariables|SetUp (Utilities|Array|Get(acopy) (Variables|Default|GetGrid) (+ (+ (LocalVariables|Geti) 1) (* (LocalVariables|Getj) (.y (Variables|Default|GetRoomSize))))))
                    (Utilities|Array|Clear (LocalVariables|GetvalidOptions))
                    (for _array_element_3 (.options (LocalVariables|GetUp))
                      (bind _output_get_4 (LocalVariables|Setvalid (Variables|/Game/Blueprints/ProceduralGeneration/Structures/BP_Tile.BP_Tile_C|GetRIGHT _array_element_3)))
                      (for _array_element_4 _output_get_4
                        (bind _returnvalue (Utilities|Array|AddUnique (LocalVariables|GetvalidOptions) _array_element_4)))
                      (bind _options1_2 (CallFunction|CheckValid (LocalVariables|GetOptions) (LocalVariables|GetvalidOptions)))
                      (LocalVariables|SetOptions _options1_2))))
                (:then_2
                  (if (< (LocalVariables|Getj) (- (.y (Variables|Default|GetRoomSize)) 1))
                    (LocalVariables|SetUp (Utilities|Array|Get(acopy) (Variables|Default|GetGrid) (+ (LocalVariables|Geti) (* (+ (LocalVariables|Getj) 1) (.y (Variables|Default|GetRoomSize))))))
                    (Utilities|Array|Clear (LocalVariables|GetvalidOptions))
                    (for _array_element_5 (.options (LocalVariables|GetUp))
                      (bind _output_get_5 (LocalVariables|Setvalid (Variables|/Game/Blueprints/ProceduralGeneration/Structures/BP_Tile.BP_Tile_C|GetDOWN _array_element_5)))
                      (for _array_element_6 _output_get_5
                        (Utilities|Array|AddUnique (LocalVariables|GetvalidOptions) _array_element_6))
                      (bind _options1_3 (CallFunction|CheckValid (LocalVariables|GetOptions) (LocalVariables|GetvalidOptions)))
                      (LocalVariables|SetOptions _options1_3))))
                (:then_3
                  (if (> (LocalVariables|Geti) 0)
                    (LocalVariables|SetUp (Utilities|Array|Get(acopy) (Variables|Default|GetGrid) (+ (- (LocalVariables|Geti) 1) (* (LocalVariables|Getj) (.y (Variables|Default|GetRoomSize))))))
                    (Utilities|Array|Clear (LocalVariables|GetvalidOptions))
                    (for _array_element_7 (.options (LocalVariables|GetUp))
                      (bind _output_get_6 (LocalVariables|Setvalid (Variables|/Game/Blueprints/ProceduralGeneration/Structures/BP_Tile.BP_Tile_C|GetLEFT _array_element_7)))
                      (for _array_element_8 _output_get_6
                        (bind _returnvalue_2 (Utilities|Array|AddUnique (LocalVariables|GetvalidOptions) _array_element_8)))
                      (bind _options1_4 (CallFunction|CheckValid (LocalVariables|GetOptions) (LocalVariables|GetvalidOptions)))
                      (LocalVariables|SetOptions _options1_4))))
                (:then_4
                  (Utilities|Array|SetArrayElem (LocalVariables|GetTMP_NextGrid) (LocalVariables|GetIndex) (Utilities|Struct|MakeBP_Cell false (LocalVariables|GetOptions) (.position (LocalVariables|GetCurrentCell)) 0)))))))
        (Variables|Default|SetGrid (LocalVariables|GetTMP_NextGrid))))
    (:then_1
      (Variables|Default|SetGrid (LocalVariables|GetTMP_NextGrid)))
    (:then_2
      (return (LocalVariables|GetTMP_NextGrid)))))

(fn CheckValid
  (params (Options :type Array%20of%20BP%20Tile%20Object%20References) (validOptions :type Array%20of%20BP%20Tile%20Object%20References))
  (bind _output_get (LocalVariables|SetTMP_OPTIONS Options))
  (for _array_element Options
    (if (not (Utilities|Array|ContainsItem validOptions _array_element))
      (Utilities|Array|RemoveItem _output_get _array_element)))
  (return (LocalVariables|GetTMP_OPTIONS)))

(fn FindCellbyPos
  (params (Grid :type Array%20of%20BP%20Cell%20Structures) (Position :type Int%20Point%20Structure))
  (bind (_x _y) (Utilities|Struct|BreakIntPoint Position))
  (bind (_array_element _array_index) (Utilities|Array|ForEachLoopwithBreak Grid)
    (:LoopBody
      (if (and (== (.X (Utilities|Struct|BreakIntPoint (.Position (Utilities|Struct|BreakBP_Cell _array_element)))) _x) (== (.Y (Utilities|Struct|BreakIntPoint (.Position (Utilities|Struct|BreakBP_Cell _array_element)))) _y))
        (return _array_element false _array_index)))
    (:Completed
      (return "" true -1))))

(fn RandomSeed
  (bind _returnvalue (Math|DateTime|UTCNow))
  (bind _randomstream (Variables|Default|GetRandomStream))
  (bind _returnvalue_2 (Class|KismetMathLibrary|RandomIntegerfromStream 1000000 _randomstream))
  (bind _returnvalue_3 (* (.year _returnvalue) (.month _returnvalue) (.day _returnvalue) (.hour _returnvalue) (.minute _returnvalue) (.second _returnvalue) (.millisecond _returnvalue)))
  (bind _returnvalue_4 (/ _returnvalue_3 _returnvalue_2))
  (if (== _returnvalue_4 0)
    (Math|Random|SetRandomStreamSeed _randomstream _returnvalue_2)
    (else
      (Math|Random|SetRandomStreamSeed _randomstream _returnvalue_4))))